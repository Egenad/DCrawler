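; Base enemy Blueprint that tracks health and handles taking damage and dying.
; AnyDamage subtracts from ActualHealth; at zero or below it frees the reserved CurrentTile and destroys the minimap representation and itself.
; Otherwise a timeline eases the LifeBar widget's percentage toward the new health ratio, feeding its Alpha into FInterpTo as DeltaTime.
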(event `self.ReceiveAnyDamage`
  (params (Damage :type "Float (single-precision)") (DamageType :type "DamageType Object Reference") (InstigatedBy :type "Controller Object Reference") (DamageCauser :type "Actor Object Reference"))
  (bind _output_get (set `self.actual_health` (- (`self.actual_health`) Damage)))
  (if (<= _output_get 0.0)
    (set `Tile.reserved` false (`self.current_tile`))
    (`self.K2_DestroyActor` (`self.minimap_representation`))
    (`self.K2_DestroyActor`)
    (else
      (bind _asenemy_health_bar_widget (cast `/Game/Source/BP/Enemy/HUD/Enemy_HealthBarWidget` (`WidgetComponent.GetWidget` (`self.life_bar`))))
      (bind (_direction _alpha) (`Timeline|Timeline_0` :!via `PlayFromStart`)
        (:`Update`
          (bind _output_get_2 (set `/Game/Source/BP/Enemy/HUD/Enemy_HealthBarWidget.Percentage` (`KismetMathLibrary.FInterpTo` (`self.last_percentage`) (/ (`self.actual_health`) (`self.max_health`)) _alpha 0.5) _asenemy_health_bar_widget))
          (set `self.last_percentage` _output_get_2))))))

(fn `UserConstructionScript`)