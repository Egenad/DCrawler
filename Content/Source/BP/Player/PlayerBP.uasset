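; Player Blueprint for a game with tile-based neighbour links, which puts the minimap on screen.
; BeginPlay creates a MinimapWidgetBP for the first player controller and adds it to the viewport.
; An unconnected debug chain would print the yaw of the interactive actor on the current tile's link to the focused tile.
; Tick, overlap and construction logic are empty.
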(event `self.ReceiveBeginPlay`
  (bind _returnvalue (`|CreateWidget` "/Game/Source/BP/Player/HUD/MinimapWidgetBP.MinimapWidgetBP_C" (`GameplayStatics.GetPlayerController` 0)))
  (`UserWidget.AddToViewport` _returnvalue 0))

(event `self.ReceiveTick`
  (params (DeltaSeconds :type "Float (single-precision)")))

(fn `UserConstructionScript`)